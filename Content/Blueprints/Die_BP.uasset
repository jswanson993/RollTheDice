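; Die actor that works out which face is pointing up and stores its number in DieUpValue every tick.
; FindUpValue picks the SidePoints component with the highest world Z, then reads the face number from its first component tag that converts to a nonzero integer.
; FirstPoint seeds the height comparison only once and is not reset here, so HighestSide carries over between ticks.
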(event `self.ReceiveTick`
  (params (DeltaSeconds :type "Float (single-precision)"))
  (bind _die_up_value (`self.Find Up Value`))
  (set `self.Die Up Value` _die_up_value))

(fn `Find Up Value`
  (returns (`Die Up Value` :type Integer))
  (locals (`Highest Side` :type "Float (double-precision)") (FirstPoint :type Boolean :default true) (`Current Top Point` :type "SceneComponent Object Reference") (Side :type Integer :default 0))
  (for _array_element (`self.SidePoints`)
    (if (`local.FirstPoint`)
      (bind (_returnvalue_x _returnvalue_y _returnvalue_z) (`KismetMathLibrary.BreakVector` (`SceneComponent.K2_GetComponentLocation` _array_element)))
      (set `local.Highest Side` _returnvalue_z)
      (set `local.Current Top Point` _array_element)
      (set `local.FirstPoint` false)
      (elif (> _returnvalue_z (`local.Highest Side`))
        (set `local.Current Top Point` _array_element)
        (set `local.Highest Side` _returnvalue_z))))
  (for _array_element_2 (`ActorComponent.ComponentTags` (`local.Current Top Point`))
    (bind _output_get (set `local.Side` (`KismetStringLibrary.Conv_StringToInt` (`KismetSystemLibrary.MakeLiteralString` (`KismetStringLibrary.Conv_NameToString` _array_element_2)))))
    (if (not (== _output_get 0))
      (return _output_get))))

(fn `UserConstructionScript`)