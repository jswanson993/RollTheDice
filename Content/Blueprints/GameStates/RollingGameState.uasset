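; Game state for a dice-rolling game that tracks level progression and which die the player rolls.
; Checkpoints are destroyed and advance the player along the Dice list, while non-checkpoint calls step back, respawning the die with a smoke puff.
; Finish pauses the game and shows a widget with strokes, die type and a score derived from side count and strokes.
; OpenNextLevel resets the die index and loads the next listed level.
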(fn `Finish`
  (params (Player :type "/Game/Blueprints/Player_BP Object Reference") (`In Finish` :type Boolean) (`Current Die` :type "/Game/Blueprints/Die/Die_BP Object Reference"))
  (returns (`Is Level Finished` :type Boolean))
  (locals (`Player Reference` :type "/Game/Blueprints/Player_BP Object Reference") (`Current Die Reference` :type "/Game/Blueprints/Die/Die_BP Object Reference"))
  (bind _strokes (`/Game/Blueprints/Player_BP.Strokes` (`local.Player Reference`)))
  (bind _returnvalue (`KismetArrayLibrary.Array_Length` (`/Game/Blueprints/Die/Die_BP.SidePoints` (`local.Current Die Reference`))))
  (set `local.Player Reference` Player)
  (set `local.Current Die Reference` `Current Die`)
  (if `In Finish`
    (set `self.Level Finished` true)
    (bind _returnvalue_2 (`|CreateWidget` "/Game/Widgets/LevelFinishWidget.LevelFinishWidget_C"))
    (`TextBlock.SetText` (`/Game/Widgets/LevelFinishWidget.RollsText` _returnvalue_2) (`KismetTextLibrary.Conv_IntToText` _strokes))
    (`TextBlock.SetText` (`/Game/Widgets/LevelFinishWidget.DieText` _returnvalue_2) (`KismetTextLibrary.Conv_StringToText` (`KismetStringLibrary.Concat_StrStr` "D" (`KismetStringLibrary.Conv_IntToString` _returnvalue))))
    (`TextBlock.SetText` (`/Game/Widgets/LevelFinishWidget.FinalScoreText` _returnvalue_2) (`KismetTextLibrary.Conv_IntToText` (`KismetMathLibrary.Clamp` (* (/ 4000 _returnvalue) (/ 1 _strokes)) 0 1000)))
    (`UserWidget.AddToViewport` _returnvalue_2 0)
    (`GameplayStatics.SetGamePaused` true)
    (return (`self.Level Finished`))
    (else
      (return false))))

(fn `OpenNextLevel`
  (if (`self.Level Finished`)
    (bind _result (`/Engine/EditorBlueprintResources/StandardMacros.IncrementInt` (`self.LevelIndex`))
      (:`  `
        (bind _output_get (set `self.LevelIndex` (`KismetMathLibrary.Clamp` _result 0 (- (`KismetArrayLibrary.Array_Length` (`self.Levels`)) 1))))
        (set `self.Level Finished` true)
        (set `self.Dice Index` 0)
        (`GameplayStatics.OpenLevel` (`|GetArrayItem` (`self.Levels`) _output_get))))))

(fn `Set New Die`
  (params (`In Checkpoint` :type Boolean) (`Current Die` :type "/Game/Blueprints/Die/Die_BP Object Reference") (Player :type "/Game/Blueprints/Player_BP Object Reference") (Checkpoint :type "/Game/Blueprints/Checkpoint_Volume_BP Object Reference"))
  (returns (`New Current Die` :type "/Game/Blueprints/Die/Die_BP Object Reference"))
  (locals (`Die Transform` :type "Transform Structure") (`Current Die Reference` :type "/Game/Blueprints/Die/Die_BP Object Reference") (`Player Refernce` :type "/Game/Blueprints/Player_BP Object Reference"))
  (bind _die_transform_location (`KismetMathLibrary.BreakTransform` (`local.Die Transform`)))
  (bind _returnvalue (+ _die_transform_location (0.0 0.0 50.0)))
  (`KismetSystemLibrary.PrintString` "Hello")
  (set `local.Current Die Reference` `Current Die`)
  (set `local.Player Refernce` Player)
  (set `local.Die Transform` (`self.GetTransform` (`local.Current Die Reference`)))
  (if `In Checkpoint`
    (`self.K2_DestroyActor` Checkpoint)
    (if (== (`self.Dice Index`) (- (`KismetArrayLibrary.Array_Length` (`self.Dice`)) 1))
      (return (`local.Current Die Reference`))
      (else
        (set `/Game/Blueprints/Player_BP.Current Die` null (`local.Player Refernce`))
        ;[1 1 1] Get the next die in the list to transform into
        (`self.K2_DestroyActor` (`local.Current Die Reference`))
        (`KismetSystemLibrary.PrintString` (`KismetStringLibrary.Conv_TransformToString` (`local.Die Transform`)))
        (bind _result (`/Engine/EditorBlueprintResources/StandardMacros.IncrementInt` (`self.Dice Index`))
          (:`  `
            (set `self.Dice Index` (`KismetMathLibrary.Clamp` _result 0 (- (`KismetArrayLibrary.Array_Length` (`self.Dice`)) 1)))))))
    (elif (== (`self.Dice Index`) 0)
      (return (`local.Current Die Reference`))
      (else
        (set `/Game/Blueprints/Player_BP.Current Die` null (`local.Player Refernce`))
        (`self.K2_DestroyActor` (`local.Current Die Reference`))
        ;[1 1 1] Get the previous die in the list to transform into
        (bind _result_2 (`/Engine/EditorBlueprintResources/StandardMacros.DecrementInt` (`self.Dice Index`))
          (:`  `
            (set `self.Dice Index` (`KismetMathLibrary.Clamp` _result_2 0 (`KismetArrayLibrary.Array_Length` (`self.Dice`)))))))))
  (`|ExecutionSequence`
    (:`then_0`
      (`NiagaraFunctionLibrary.SpawnSystemAtLocation` "/Game/Particles/SmokePuff/SmokePuff.SmokePuff" _returnvalue (struct) (4.0 4.0 4.0)))
    (:`then_1`
      (bind _returnvalue_2 (`|SpawnActorFromClass` (`|GetArrayItem` (`self.Dice`) (`self.Dice Index`)) (`KismetMathLibrary.MakeTransform` _returnvalue) "Undefined" "OverrideRootScale" null null))
      (set `/Game/Blueprints/Player_BP.Current Die` _returnvalue_2 (`local.Player Refernce`))
      (return _returnvalue_2))))

(fn `UserConstructionScript`)