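; Player pawn for a dice-throwing game: grabs, shakes and throws a physics die with the mouse, counting each throw as a stroke.
; Grab traces under the cursor and attaches a PhysicsHandle; release marks the die Thrown.
; While held, the target combines a camera-forward trace hit, centered cursor offset, shake height and amplified mouse delta, with debug drawing.
; Otherwise the root follows the current die, and right-mouse drag yaws the camera.
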(event `self.ReceiveBeginPlay`
  (set `PlayerController.bShowMouseCursor` true (`GameplayStatics.GetPlayerController` 0)))

(event `self.ReceiveTick`
  (params (DeltaSeconds :type "Float (single-precision)"))
  (bind _dragged_component (`self.Dragged Component`))
  (bind (_deltax _deltay) (`PlayerController.GetInputMouseDelta` (`GameplayStatics.GetPlayerController` 0)))
  (bind (_returnvalue_x _returnvalue_y _returnvalue_z) (`KismetMathLibrary.BreakVector` (+ (`self.TranslateMouseXY`) (* (`KismetMathLibrary.MakeVector` _deltay _deltax) (`self.Shake Intensity`)))))
  (if (`self.Grabbed`)
    (`/Engine/EditorBlueprintResources/StandardMacros.IsValid` _dragged_component
      (:`Is Valid`
        (if (`SceneComponent.IsSimulatingPhysics` _dragged_component "None")
          (`PhysicsHandleComponent.SetTargetLocation` (`self.PhysicsHandle`) (`KismetMathLibrary.MakeVector` _returnvalue_x _returnvalue_y _returnvalue_z))
          (`KismetSystemLibrary.DrawDebugLine` (`KismetMathLibrary.TransformLocation` (`SceneComponent.K2_GetComponentToWorld` (`self.Dragged Component`)) (`self.Relative Grab Location`)) (`KismetMathLibrary.MakeVector` _returnvalue_x _returnvalue_y _returnvalue_z) (struct :`R` 0.572917 :`G` 0.028268 :`B` 0.005466 :`A` 1.0) 0.0 5.0))))
    (else
      (`SceneComponent.K2_SetWorldLocation` (`self.DefaultSceneRoot`) (`SceneComponent.K2_GetComponentLocation` (`/Game/Blueprints/Die_BP.Center` (`self.Current Die`))) false true))))

(event `Key|RightMouseButton`
  (params (Key :type "Key Structure"))
  (:`Pressed`
    (set `self.Camera Rotation` true))
  (:`Released`
    (set `self.Camera Rotation` false)))

(event `InputAxisKey|MouseX`
  (params (AxisValue :type "Float (single-precision)"))
  (if (`self.Camera Rotation`)
    (`SceneComponent.K2_AddWorldRotation` (`self.DefaultSceneRoot`) (`KismetMathLibrary.MakeRotator` 0.0 0.0 (* AxisValue (`self.Camera Rotate Speed`))) false false)))

(event `InputAction|Grab`
  (params (Key :type "Key Structure"))
  (bind (_worldlocation _worlddirection) (`PlayerController.DeprojectMousePositionToWorld` (`GameplayStatics.GetPlayerController` 0)))
  (bind (_worldlocation_2 _worlddirection_2) (`PlayerController.DeprojectMousePositionToWorld` (`GameplayStatics.GetPlayerController` 0)))
  (:`Pressed`
    (if (not (`/Game/Blueprints/Die_BP.Thrown` (`self.Current Die`)))
      (`KismetSystemLibrary.DrawDebugSphere` (+ _worldlocation_2 (* _worlddirection_2 10.0)) 0.5 12 (struct :`R` 1.0 :`G` 0.180501 :`A` 1.0) 1000.0 1.0)
      (bind (_outhit _returnvalue) (`KismetSystemLibrary.LineTraceSingle` :`Start` _worldlocation :`End` (+ _worldlocation (* _worlddirection 10000.0)) :`TraceChannel` "TraceTypeQuery1" :`bTraceComplex` true :`DrawDebugType` "ForDuration" :`DrawTime` 0.0))
      (if _returnvalue
        (bind (_bblockinghit _binitialoverlap _time _distance _location _impactpoint _normal _impactnormal _physmat _hitactor _hitcomponent) (`GameplayStatics.BreakHitResult` _outhit))
        (set `self.Initial Distance To Component` _distance)
        (bind _asdie_bp (cast `/Game/Blueprints/Die_BP` _hitactor))
        (bind _output_get (set `self.Current Die` _asdie_bp))
        (set `self.Dragged Component` (`/Game/Blueprints/Die_BP.DieBody` _output_get))
        (if (`SceneComponent.IsSimulatingPhysics` _hitcomponent "None")
          (`PhysicsHandleComponent.GrabComponentAtLocation` (`self.PhysicsHandle`) (`self.Dragged Component`) "None" _location)
          (set `self.Grabbed` true)
          (set `self.Relative Grab Location` (`KismetMathLibrary.InverseTransformLocation` (`SceneComponent.K2_GetComponentToWorld` (`self.Dragged Component`)) _location))))))
  (:`Released`
    (if (`self.Grabbed`)
      (set `/Game/Blueprints/Die_BP.Thrown` true (`self.Current Die`))
      (`/Engine/EditorBlueprintResources/StandardMacros.IncrementInt` (`self.Strokes`)
        (:`  `
          (set `self.Grabbed` false)
          (set `self.Dragged Component` null)
          (`PhysicsHandleComponent.ReleaseComponent` (`self.PhysicsHandle`)))))))

(fn `GetMouseXYCentered`
  (returns (X :type "Float (double-precision)") (Y :type "Float (double-precision)"))
  (bind (_returnvalue_x _returnvalue_y) (`KismetMathLibrary.BreakVector2D` (`WidgetLayoutLibrary.GetViewportSize`)))
  (bind (_locationx _locationy) (`PlayerController.GetMousePosition` (`GameplayStatics.GetPlayerController` 0)))
  (bind _result (`/Engine/EditorBlueprintResources/StandardMacros.NegateFloat` (- _locationy (/ _returnvalue_y 2.0)))
    (:`  `
      (return (- _locationx (/ _returnvalue_x 2.0)) _result))))

(fn `TranslateMouseXY`
  (returns (`Mouse Position` :type "Vector Structure"))
  (bind (_x _y) (`self.GetMouseXYCentered`))
  (bind _camera (`self.Camera`))
  (bind _returnvalue (`SceneComponent.K2_GetComponentLocation` _camera))
  (bind _outhit (`KismetSystemLibrary.LineTraceSingle` _returnvalue (+ _returnvalue (* (`SceneComponent.GetForwardVector` _camera) 1000.0)) "TraceTypeQuery1" true (`|MakeArray` (`self.Current Die`) :!type "Actor Object Reference") "ForOneFrame"))
  (bind _returnvalue_2 (+ (`KismetMathLibrary.MakeVector` _y _x (`self.Shake Height`)) (`.Location` (`GameplayStatics.BreakHitResult` _outhit))))
  (`KismetSystemLibrary.DrawDebugSphere` _returnvalue_2 100.0 12 (struct :`R` 1.0 :`G` 0.180501 :`A` 1.0) 0.0 50.0)
  (return _returnvalue_2))

(fn `UserConstructionScript`)