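; Goblin archer enemy that fires D20 projectiles continuously from its Arrow component's location, with no targeting logic.
; On BeginPlay, a looping timer spawns a projectile at the ArrowSpawnRate interval and appends it to ProjectileArray.
; After a short delay, a second timer at the same interval destroys and removes the oldest entry, acting as a first-in, first-out lifetime limit.
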(event `self.ReceiveBeginPlay`
  (bind _returnvalue (`KismetMathLibrary.Conv_IntToDouble` (`self.Arrow_Spawn_Rate`)))
  (`KismetSystemLibrary.K2_SetTimer` null "SpawnProjectile" _returnvalue true)
  (`KismetSystemLibrary.Delay` 4.0)
  (`KismetSystemLibrary.K2_SetTimer` null "DestroyProjectile" _returnvalue true))

(fn `DestroyProjectile`
  (locals (ProjectileToDestroy :type "Actor Object Reference"))
  (bind _projectilearray (`self.ProjectileArray`))
  (`self.K2_DestroyActor` (`|GetArrayItem` _projectilearray))
  (`KismetArrayLibrary.Array_Remove` _projectilearray))

(fn `SpawnProjectile`
  (bind _returnvalue (`|SpawnActorFromClass` "/Game/BluePrints/Die/D20_Projectile_BP.D20_Projectile_BP_C" (`KismetMathLibrary.MakeTransform` (`SceneComponent.K2_GetComponentLocation` (`self.Arrow`))) "AdjustIfPossibleButAlwaysSpawn" "OverrideRootScale" null null))
  (`KismetArrayLibrary.Array_Add` (`self.ProjectileArray`) _returnvalue))

(fn `UserConstructionScript`)