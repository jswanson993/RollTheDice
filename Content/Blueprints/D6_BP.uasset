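; D6_BP is a six-sided die Blueprint that supplies its face markers to a parent class.
; Its construction script runs the parent's script, then fills SidePoints with Number1 through Number6 in order.
; Tick only forwards to the parent, and BeginPlay and overlap are disabled stubs, so any die behavior lives outside this graph.
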(event `self.ReceiveTick`
  (params (DeltaSeconds :type "Float (single-precision)"))
  (`parent.ReceiveTick` DeltaSeconds))

(fn `UserConstructionScript`
  (`parent.UserConstructionScript`)
  (set `self.SidePoints` (`|MakeArray` (`self.Number 1`) (`self.Number 2`) (`self.Number 3`) (`self.Number 4`) (`self.Number 5`) (`self.Number 6`))))