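; Physics die actor that reports which face is up and alerts the level Blueprint when a throw comes to rest.
; Each tick it derives the value from the highest socket on DieBody, parsing the socket name's suffix.
; It also applies a zero force to avoid sticking and fires the stop notification once velocity nears zero.
; Hits play wood impact sounds scaled by impulse, filtered by strength and distance from the previous impact.
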(event `self.ReceiveTick`
  (params (DeltaSeconds :type "Float (single-precision)"))
  (bind _die_up_value (`self.Find Up Value`))
  (set `self.Die Up Value` _die_up_value)
  ;[1 1 1] Die will get stuck if there isnt a force being applied
  (`PrimitiveComponent.AddForce` (`self.DieBody`) (0.0 0.0 0.0) "None" false)
  ;[1 1 1] Check to see if the die has stopped moving after thrown and alert the level blueprint if so
  (if (and (`self.Thrown`) (== (`self.GetVelocity`) (0.0 0.0 0.0) :`ErrorTolerance` 0.5))
    (set `self.Thrown` false)
    (`self.NotifyMovementStopped`)))

(event `self.DieBody.OnComponentHit`
  (params (HitComponent :type "PrimitiveComponent Object Reference") (OtherActor :type "Actor Object Reference") (OtherComp :type "PrimitiveComponent Object Reference") (NormalImpulse :type "Vector Structure") (Hit :type "HitResult Structure (by ref)"))
  (bind _returnvalue (`KismetMathLibrary.VSize` NormalImpulse))
  (bind _impactsoundthreshold (`self.impactSoundThreshold`))
  (if (and (> (`KismetMathLibrary.Vector_Distance` (`self.previousImpactPoint`) Hit_ImpactPoint) 50.0) (> _returnvalue _impactsoundthreshold))
    (`GameplayStatics.PlaySoundAtLocation` "/Game/Audio/SFX/WoodHit_CUE.WoodHit_CUE" Hit_Location (struct) (`KismetMathLibrary.FClamp` (/ (- _returnvalue _impactsoundthreshold) (* _impactsoundthreshold 3.0))) 1.0 0.0 null null null null)
    (set `self.previousImpactPoint` Hit_ImpactPoint)))

(fn `Find Up Value`
  (returns (`Die Up Value` :type Integer))
  (locals (`Highest Side` :type "Float (double-precision)") (FirstPoint :type Boolean :default true) (`Current Top Point` :type "SceneComponent Object Reference") (Side :type Integer :default 0) (TopSocket :type Name))
  (for _array_element (`SceneComponent.GetAllSocketNames` (`self.DieBody`))
    (bind (_returnvalue_x _returnvalue_y _returnvalue_z) (`KismetMathLibrary.BreakVector` (`SceneComponent.GetSocketLocation` (`self.DieBody`) _array_element)))
    (if (> _returnvalue_z (`local.Highest Side`))
      (set `local.Highest Side` _returnvalue_z)
      (set `local.TopSocket` _array_element)))
  (bind _output_get (set `local.Side` (`KismetStringLibrary.Conv_StringToInt` (`.RightS` (`KismetStringLibrary.Split` (`KismetStringLibrary.Conv_NameToString` (`local.TopSocket`)) "_")))))
  (return (+ _output_get 1)))

(fn `UserConstructionScript`)